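; Player character Blueprint for a melee fighter with running, sword attack, shield block, health and death.
; Tick polls input to set walk speed and toggle sword and shield collision while mouse buttons are held, reattaches both colliders to mesh sockets, and caps health.
; Capsule overlaps subtract Enemy_Blueprint damage, pausing with a game-over widget at zero health.
; Shield overlaps with tagged AI weapons launch the player along the attacker's forward vector.
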(event `self.ReceiveBeginPlay`
  (`self.Player_Value_Set_Up`))

(event `self.ReceiveTick`
  (params (DeltaSeconds :type "Float (single-precision)"))
  ;[1 1 1] Update
  (`self.PlayerRun`)
  (`self.Animation_SwordCollisionDetection`)
  (`self.TurnOffColliderComponents`)
  ;[1 1 1] Max Health Check
  (if (> (`self.CurrentHealth`) (`self.maxHealth`))
    (set `self.CurrentHealth` (`self.maxHealth`))
    (else
      (set `self.CurrentHealth` (`self.CurrentHealth`)))))

(event `self.CapsuleComponent.OnComponentBeginOverlap`
  (params (OverlappedComponent :type "PrimitiveComponent Object Reference") (OtherActor :type "Actor Object Reference") (OtherComp :type "PrimitiveComponent Object Reference") (OtherBodyIndex :type Integer) (bFromSweep :type Boolean) (SweepResult :type "HitResult Structure (by ref)"))
  ;[1 1 1] Player detect component attach to the AI which applies damage
  (`/Engine/EditorBlueprintResources/StandardMacros.DoOnce` false :!label _label
    (:`Completed`
      (`self.Player_Health` OtherActor)
      (`self.DamageRestter`))))

(event `DamageRestter`
  ;[1 1 1] Player detect component attach to the AI which applies damage
  (goto _label :!via `Reset`))

(event `self.ShieldCollision.OnComponentBeginOverlap`
  (params (OverlappedComponent :type "PrimitiveComponent Object Reference") (OtherActor :type "Actor Object Reference") (OtherComp :type "PrimitiveComponent Object Reference") (OtherBodyIndex :type Integer) (bFromSweep :type Boolean) (SweepResult :type "HitResult Structure (by ref)"))
  ;[1 1 1] Condition that says has the right tagged hit the shield
  (if (`ActorComponent.ComponentHasTag` OtherComp (`self.AI_Weapon_Tag`))
    ;[1 1 1] Push player back
    (`self.LaunchCharacter` (* (`KismetMathLibrary.GetForwardVector` (`self.K2_GetActorRotation` OtherActor)) (`self.knockBack_Force`)))))

(fn `Animation_SwordCollisionDetection`
  (`SceneComponent.K2_AttachToComponent` (`self.SwordHitCollision`) (`self.Mesh`) "Sword_joint" "KeepWorld" "KeepWorld" "KeepWorld" true)
  (`SceneComponent.K2_AttachToComponent` (`self.ShieldCollision`) (`self.Mesh`) "Shield_joint" "KeepWorld" "KeepWorld" "KeepWorld" true))

(fn `Player_Health`
  (params (enemyHit :type "Actor Object Reference"))
  (bind _returnvalue (`GameplayStatics.GetPlayerController` 0))
  ;[1 1 1] Enemy Hit will be the enemy that hit us on the overlap collision
  ;[1 1 1] Get the enemy
  (bind _asenemy_blueprint (cast `/Game/BluePrints/NPCs/Enemy_Blueprint` enemyHit))
  ;[1 1 1] Set New Health value
  (bind _output_get (set `self.currentHealth` (- (`self.currentHealth`) (`/Game/BluePrints/NPCs/Enemy_Blueprint.Current_Damage` _asenemy_blueprint))))
  ;[1 1 1] Is The Player Dead? Health <= 0 = death
  (`KismetSystemLibrary.PrintString` (`KismetStringLibrary.Conv_IntToString` _output_get))
  (if (<= (`self.currentHealth`) 0)
    (set `self.player_Dead` true)
    ;[1 1 1] Show Game Over Screen
    (bind _returnvalue_2 (`|CreateWidget` "/Game/BluePrints/Menus/GameOver_BP.GameOver_BP_C"))
    (`UserWidget.AddToViewport` _returnvalue_2 0)
    (`self.DisableInput` (`GameplayStatics.GetPlayerCharacter` 0) _returnvalue)
    (set `PlayerController.bShowMouseCursor` true _returnvalue)
    (`GameplayStatics.SetGamePaused` true)
    (else
      (set `self.currentHealth` (`self.currentHealth`)))))

(fn `Player_Value_Set_Up`
  ;[1 1 1] Set Up Health
  (set `self.CurrentHealth` (`self.maxHealth`))
  ;[1 1 1] Set up the damage of attacks and run key
  (set `self.current_Damage` 10)
  (set `self.Run Key` "R")
  ;[1 1 1] Update Health Bar on begin play
  (message `/Game/BluePrints/Player/UI/Interface/BPI_Player.Update_HealthBar` self (/ (`KismetMathLibrary.Conv_IntToDouble` (`self.CurrentHealth`)) (`KismetMathLibrary.Conv_IntToDouble` (`self.maxHealth`)))))

(fn `PlayerRun`
  (locals (NewLocalVar_0 :type "RadialFalloff Object Reference"))
  (bind _charactermovement (`self.CharacterMovement`))
  (if (`PlayerController.IsInputKeyDown` (`GameplayStatics.GetPlayerController` 0) (`self.Run Key`))
    ;[1 1 1] We Are Running
    (set `self.accelerationSpeed` (`self.Acceleration_Speed`))
    (set `CharacterMovementComponent.MaxWalkSpeed` (`self.accelerationSpeed`) _charactermovement)
    (else
      ;[1 1 1] We Are Walking
      (set `self.defaultSpeed` (`self.defualtSpeed`))
      (set `CharacterMovementComponent.MaxWalkSpeed` (`self.defaultSpeed`) _charactermovement))))

(fn `TurnOffColliderComponents`
  (locals (LeftMouse :type "Key Structure" :default "LeftMouseButton") (RightMouse :type "Key Structure" :default "RightMouseButton") (AttackingEnable :type Boolean) (BlockingEnable :type Boolean))
  ;[1 1 1] Sword Collision on or Off
  ;;[1 1 1] Monitor the 2 states if the player is getting input down or not
  (if (> (`PlayerController.GetInputKeyTimeDown` (`GameplayStatics.GetPlayerController` 0) "LeftMouseButton") 0.0)
    (set `local.AttackingEnable` true)
    (else
      (set `local.AttackingEnable` false)))
  ;;[1 1 1] After gathering what the player has done turn off or on collider depending on data
  (if (`local.AttackingEnable`)
    (`PrimitiveComponent.SetCollisionEnabled` (`self.SwordHitCollision`) "QueryOnly")
    (else
      (`PrimitiveComponent.SetCollisionEnabled` (`self.SwordHitCollision`) "NoCollision")))
  ;[1 1 1] Repeat Same process shown for sword to turn off sheidl
  (if (> (`PlayerController.GetInputKeyTimeDown` (`GameplayStatics.GetPlayerController` 0) "RightMouseButton") 0.0)
    (set `local.BlockingEnable` true)
    (else
      (set `local.BlockingEnable` false)))
  (if (`local.BlockingEnable`)
    (`PrimitiveComponent.SetCollisionEnabled` (`self.ShieldCollision`) "QueryOnly")
    (else
      (`PrimitiveComponent.SetCollisionEnabled` (`self.ShieldCollision`) "NoCollision"))))

(fn `UserConstructionScript`)