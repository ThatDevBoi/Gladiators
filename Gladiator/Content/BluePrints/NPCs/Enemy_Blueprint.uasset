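; Melee enemy NPC Blueprint that chases the player, swipes on arrival and can die.
; BeginPlay sets up health, attaches a sphere to the left forearm and starts a recursive AIMoveTo chase-attack loop using directly played animations.
; Any capsule overlap subtracts CurrentDamage, but death animation and destruction run only after the next successful move's attack delay.
; Weapon overlaps just print; random roaming exists but is never started, and TakeDamage is empty.
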(event `self.ReceiveBeginPlay`
  ;[1 1 1] Before play set up NPC Health
  (`self.Chase`)
  (`self.WeaponCollider_FollowAnimation`)
  (`self.SetUp_Health`))

(event `self.CapsuleComponent.OnComponentBeginOverlap`
  (params (OverlappedComponent :type "PrimitiveComponent Object Reference") (OtherActor :type "Actor Object Reference") (OtherComp :type "PrimitiveComponent Object Reference") (OtherBodyIndex :type Integer) (bFromSweep :type Boolean) (SweepResult :type "HitResult Structure (by ref)"))
  ;[1 1 1] Damage and death message
  (set `self.currentHealth` (- (`self.currentHealth`) (`self.Current_Damage`)))
  (`KismetSystemLibrary.PrintString` (`KismetStringLibrary.Conv_IntToString` (`self.currentHealth`)))
  (if (<= (`self.currentHealth`) 0)
    (`KismetSystemLibrary.PrintString` "Enemy_Dead")
    (set `self.imDead` true)
    (else
      (set `self.currentHealth` (`self.currentHealth`)))))

(event `self.Enemy_Weapon_Collision.OnComponentBeginOverlap`
  (params (OverlappedComponent :type "PrimitiveComponent Object Reference") (OtherActor :type "Actor Object Reference") (OtherComp :type "PrimitiveComponent Object Reference") (OtherBodyIndex :type Integer) (bFromSweep :type Boolean) (SweepResult :type "HitResult Structure (by ref)"))
  (`KismetSystemLibrary.PrintString` "Hit Shield"))

(event `Roam`
  ;[1 1 1] Roaming
  (`|AIMoveTo` self (`NavigationSystemV1.K2_GetRandomLocationInNavigableRadius` (`self.K2_GetActorLocation`) 500.0 null null) null
    (:`then`
      (`KismetSystemLibrary.Delay` (`self.DelayForRoam`))
      (`self.Roam`))))

(event `Chase`
  ;[1 1 1] AI Can chase the player by getting the players position
  ;;[1 1 1] Play running animation on start
  (`SkeletalMeshComponent.PlayAnimation` (`self.Mesh`) "/Game/Mesh/NPCMesh/Animations/Movement/Running_Anim_mixamo_com.Running_Anim_mixamo_com" true)
  ;;[1 1 1] Move towards player
  (`|AIMoveTo` self (0.0 0.0 0.0) (`GameplayStatics.GetPlayerPawn` 0)
    (:`OnSuccess`
      ;;[1 1 1] Attack player when close
      (`SkeletalMeshComponent.PlayAnimation` (`self.Mesh`) "/Game/Mesh/NPCMesh/Animations/Combat/Mutant_Swiping_mixamo_com.Mutant_Swiping_mixamo_com" false)
      (`KismetSystemLibrary.Delay` (`self.DelayForChase`))
      ;;[1 1 1] Is this object Dead?
      (if (`self.imDead`)
        (`SkeletalMeshComponent.PlayAnimation` (`self.Mesh`) "/Game/Mesh/NPCMesh/Animations/Combat/Mutant_Dying.Mutant_Dying" false)
        (`KismetSystemLibrary.Delay` 4.0)
        (`self.K2_DestroyActor`)
        (else
          (`self.Chase`))))))

(fn `SetUp_Health`
  ;[1 1 1] Sets up AI Health on start
  (set `self.Max_Health` (`self.Max_Health`))
  (set `self.Current_Damage` (`self.Current_Damage`))
  (set `self.currentHealth` (`self.Max_Health`)))

(fn `TakeDamage`)

(fn `UserConstructionScript`)

(fn `WeaponCollider_FollowAnimation`
  (`SceneComponent.K2_AttachToComponent` (`self.Sphere`) (`self.Mesh`) "LeftForeArm" "KeepWorld" "KeepWorld" "KeepWorld" true))