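; Mutant spawner that keeps the world stocked with Enemy_Blueprint AI up to the EnemiesToSpawn limit.
; Every Tick it rolls an easy, medium or hard tier, each with its own health, damage and points on death.
; SpawnActor counts all enemies in the world and, if below the limit, spawns one at SpawnerBox and applies that tier's stats.
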(event `self.ReceiveBeginPlay`
  ;[1 1 1] Before Game Starts
  (`self.Set_Up_Values`))

(event `self.ReceiveTick`
  (params (DeltaSeconds :type "Float (single-precision)"))
  ;[1 1 1] Every Frame
  (`self.Multi_AI_Spawner`))

(event `Multi_AI_Spawner`
  ;[1 1 1] Depending on the value that generates randomly
  (switch `int` (`KismetMathLibrary.RandomIntegerInRange` 0 2)
    (:`0`
      ;[1 1 1] Easy
      (`self.Spawn_Actor` (`self.Easy_Health`) 10 50 100))
    (:`1`
      ;[1 1 1] Medium
      (`self.Spawn_Actor` (`self.Medium_Health_Increase`) 15 100 150))
    (:`2`
      ;[1 1 1] Hard
      (`self.Spawn_Actor` (`self.Hard_Health_Increase`) 20 200 200))))

(fn `Set_Up_Values`
  (set `self.Easy_Health` 100)
  (set `self.Medium_Health_Increase` 150)
  (set `self.Hard_Health_Increase` 200))

(fn `Spawn_Actor`
  (params (HealthChanger :type Integer) (Damage_Changer :type Integer) (PointChanger :type Integer) (maxHealth :type Integer))
  ;[0.9948 0.9896 1 1 16] Health Changer value takes into mind what health the Actor enemy spawns with which is set in Event Graph: Damage changer changes the damage of the Enemy. so that the damage the player recives changes
  ;[1 1 1] Find the enemy class we want to spawn and continue to spawn them depending on the value we can set
  ;;[1 1 1] Find actors class
  (bind _outactors (`GameplayStatics.GetAllActorsOfClass` "/Game/BluePrints/NPCs/Enemy_Blueprint.Enemy_Blueprint_C"))
  ;;[1 1 1] Spawn the enemies depending on the enemies to spawn value
  (if (< (`KismetArrayLibrary.Array_Length` _outactors) (`self.Enemies_ToSpawn`))
    (bind _returnvalue (`AIBlueprintHelperLibrary.SpawnAIFromClass` "/Game/BluePrints/NPCs/Enemy_Blueprint.Enemy_Blueprint_C" null (`SceneComponent.K2_GetComponentLocation` (`self.SpawnerBox`))))
    ;[1 1 1] When the actor has spawned make sure it spawns with the correct health
    (bind _asenemy_blueprint (cast `/Game/BluePrints/NPCs/Enemy_Blueprint` _returnvalue))
    (set `/Game/BluePrints/NPCs/Enemy_Blueprint.currentHealth` HealthChanger _asenemy_blueprint)
    (set `/Game/BluePrints/NPCs/Enemy_Blueprint.Max_Health` maxHealth _asenemy_blueprint)
    (set `/Game/BluePrints/NPCs/Enemy_Blueprint.Current_Damage` Damage_Changer _asenemy_blueprint)
    (set `/Game/BluePrints/NPCs/Enemy_Blueprint.Points_On_Death` PointChanger _asenemy_blueprint)))

(fn `UserConstructionScript`)